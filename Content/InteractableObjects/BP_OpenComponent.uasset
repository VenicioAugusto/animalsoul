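; Character component for interacting with openable objects, currently a partial implementation.
; BeginInteraction plays a pushing montage on the owning Character when animation is requested and CurrentOpenable is invalid.
; IsInteractingWithObject reports whether CurrentOpenable is valid, but nothing here assigns it or uses the passed InteractableObject.
; EndInteraction is empty, and the logic constraining movement to a plane and disabling orient-to-movement is disconnected.
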(fn `BeginInteraction`
  (params (InteractableObject :type "/Game/InteractableObjects/BP_InteractableObject Object Reference") (HasAnimation :type Boolean))
  (locals (OwningCharacter :type "Character Object Reference"))
  (if HasAnimation
    (if (not (`KismetSystemLibrary.IsValid` (`self.CurrentOpenable`)))
      (bind _ascharacter (cast `Character` (`self.GetOwner`)))
      (bind _output_get (set `local.OwningCharacter` _ascharacter))
      (`Character.PlayAnimMontage` _output_get "/Game/SideScroller/Animations/FromNewMixamo/Pushing_Retargeted_Montage.Pushing_Retargeted_Montage" 1.0 "None"))))

(fn `EndInteraction`)

(fn `IsInteractingWithObject`
  (returns (ReturnValue :type Boolean))
  (return (`KismetSystemLibrary.IsValid` (`self.CurrentOpenable`))))
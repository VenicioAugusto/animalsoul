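; Base interactable object that a character with BP_OpenComponent can toggle open or closed.
; Interaction requires the side-scroller character inside CanOpenArea and respects lock and open-once flags.
; When movement is needed, it snaps the character to the nearest in-range OpenTransform, previewed by construction-script arrows, after traces confirm room, walkable floor and no wall.
; It then calls BeginInteracting on the component and flips OpenClosedState, printing debug feedback.
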(event `self.ReceiveBeginPlay`)

(event `/Game/SideScroller/IN_SideScroller.OnInteractedIN`
  (params (Player :type "/Game/SideScroller/BP_SideScrollerCharacter Object Reference"))
  (`self.HandleInteraction` Player))

(event `self.CanOpenArea.OnComponentBeginOverlap`
  (params (OverlappedComponent :type "PrimitiveComponent Object Reference") (OtherActor :type "Actor Object Reference") (OtherComp :type "PrimitiveComponent Object Reference") (OtherBodyIndex :type Integer) (bFromSweep :type Boolean) (SweepResult :type "HitResult Structure (by ref)"))
  (cast `/Game/SideScroller/BP_SideScrollerCharacter` OtherActor)
  (set `self.IsInTheOpenArea?` true))

(event `self.CanOpenArea.OnComponentEndOverlap`
  (params (OverlappedComponent :type "PrimitiveComponent Object Reference") (OtherActor :type "Actor Object Reference") (OtherComp :type "PrimitiveComponent Object Reference") (OtherBodyIndex :type Integer))
  (cast `/Game/SideScroller/BP_SideScrollerCharacter` OtherActor)
  (set `self.IsInTheOpenArea?` false))

(fn `AnimationVerification`
  (returns (`HasAnimation?` :type Boolean))
  (return (`self.HasAnimation?`)))

(fn `FindClosestPushTransformIndex`
  (params (CharacterLocation :type "Vector2D Structure") (InteractRange :type "Float (double-precision)"))
  (returns (BestIndex :type Integer))
  (locals (CurrentTransformIndex :type Integer) (CurrentDiscanteSqr :type "Float (double-precision)") (ClosestTransformIndex :type Integer) (ClosestDistanceSqr :type "Float (double-precision)"))
  (for (_array_element _array_index) (`self.OpenTransforms`)
    (set `local.CurrentTransformIndex` _array_index)
    (bind _output_get (set `local.CurrentDiscanteSqr` (`KismetMathLibrary.DistanceSquared2D` (`KismetMathLibrary.Conv_VectorToVector2D` (`KismetMathLibrary.TransformLocation` (`self.GetTransform`) (.location _array_element))) (`local.CharacterLocation`))))
    (if (< _output_get (`KismetMathLibrary.Square` (`local.InteractRange`)))
      (if (or (< (`local.CurrentDiscanteSqr`) (`local.ClosestDistanceSqr`)) (< (`local.ClosestTransformIndex`) 0))
        (set `local.ClosestTransformIndex` (`local.CurrentTransformIndex`))
        (set `local.ClosestDistanceSqr` (`local.CurrentDiscanteSqr`)))))
  (return (`local.ClosestTransformIndex`)))

(fn `HandleInteraction`
  (params (Character :type "Character Object Reference"))
  (locals (OpenComponent :type "/Game/InteractableObjects/BP_OpenComponent Object Reference") (CharacterNewTransform :type "Transform Structure"))
  (bind _characternewtransform_location (`KismetMathLibrary.BreakTransform` (`local.CharacterNewTransform`)))
  (bind _characternewtransform_location_2 (`KismetMathLibrary.BreakTransform` (`local.CharacterNewTransform`)))
  (bind _capsulecomponent (`Character.CapsuleComponent` (`local.Character`)))
  (`/Engine/EditorBlueprintResources/StandardMacros.IsValid` Character
    (:`Is Valid`
      (bind _output_get (set `local.OpenComponent` (`self.GetComponentByClass` Character "/Game/InteractableObjects/BP_OpenComponent.BP_OpenComponent_C")))
      (`/Engine/EditorBlueprintResources/StandardMacros.IsValid` _output_get
        (:`Is Valid`
          (if (`self.IsInTheOpenArea?`)
            (if (not (`self.IsLocked?`))
              (if (not (and (`self.IsDoOnce?`) (`self.OpenClosedState`)))
                (if (`self.NeedToMove?`)
                  (bind _bestindex (`self.FindClosestPushTransformIndex` (`KismetMathLibrary.Conv_VectorToVector2D` (`self.K2_GetActorLocation` (`local.Character`))) (`/Game/InteractableObjects/BP_OpenComponent.InteractRange` (`local.OpenComponent`))))
                  (if (>= _bestindex 0)
                    (bind (_returnvalue_location _returnvalue_rotation) (`KismetMathLibrary.BreakTransform` (`KismetMathLibrary.ComposeTransforms` (`|GetArrayItem` (`self.OpenTransforms`) _bestindex) (`self.GetTransform`))))
                    (bind _output_get_2 (set `local.CharacterNewTransform` (`KismetMathLibrary.MakeTransform` (+ _returnvalue_location (`KismetMathLibrary.MakeVector` 0.0 0.0 (`CapsuleComponent.GetScaledCapsuleHalfHeight` (`Character.CapsuleComponent` (`local.Character`))))) _returnvalue_rotation)))
                    (`KismetSystemLibrary.DrawDebugSphere` (.location _output_get_2) 20.0 12 (struct :`R` 1.0 :`B` 0.081321 :`A` 1.0) 2.0 1.0)
                    (bind _outhit (`KismetSystemLibrary.CapsuleTraceSingle` (+ _characternewtransform_location (0.0 0.0 70.0)) (- _characternewtransform_location (0.0 0.0 100.0)) (`CapsuleComponent.GetScaledCapsuleRadius` _capsulecomponent) (`CapsuleComponent.GetScaledCapsuleHalfHeight` _capsulecomponent) "TraceTypeQuery1"))
                    (bind (_bblockinghit _binitialoverlap _time _distance _location _impactpoint _normal _impactnormal) (`GameplayStatics.BreakHitResult` _outhit))
                    (if (not _binitialoverlap)
                      (if (< (`CharacterMovementComponent.K2_GetWalkableFloorZ` (`Character.CharacterMovement` (`local.Character`))) (.z _impactnormal))
                        (bind (_outhit_2 _returnvalue) (`KismetSystemLibrary.LineTraceSingle` (`self.K2_GetActorLocation`) _characternewtransform_location_2 "TraceTypeQuery1" false (`|MakeArray` (`local.Character`) :!type "Actor Object Reference") "ForDuration" true (struct :`R` 1.0 :`A` 1.0) (struct :`G` 1.0 :`A` 1.0) 2.0))
                        (if (not _returnvalue)
                          (`self.K2_SetActorTransform` (`local.Character`) (`local.CharacterNewTransform`) false false)
                          (`/Game/InteractableObjects/BP_OpenComponent.BeginInteracting` (`local.OpenComponent`) self :!label _label)
                          (bind _openclosedstate (`self.OpenAndClose`))
                          (`KismetSystemLibrary.PrintString` (`KismetStringLibrary.Conv_BoolToString` _openclosedstate))
                          (else
                            (`self.PushFailedInfo` "Wall between character and object.")))
                        (else
                          (`self.PushFailedInfo` "Floor not walkable.")))
                      (else
                        (`self.PushFailedInfo` "No room to stand.")))
                    (else
                      (`self.PushFailedInfo` "No Interact tranform found.")))
                  (else
                    (goto _label)))
                (else
                  (`KismetSystemLibrary.PrintString` "Its Already Open!")))
              (else
                (`KismetSystemLibrary.PrintString` "Its Locked!")))))
        (:`Is Not Valid`
          (`self.PushFailedInfo` "Character does not have OpenComponent"))))
    (:`Is Not Valid`
      (`self.PushFailedInfo` "Character is Invalid."))))

(fn `OpenAndClose`
  (returns (OpenClosedState :type Boolean))
  (locals (CurrentOpenCloseState :type Boolean))
  (bind _output_get (set `local.CurrentOpenCloseState` (`self.OpenClosedState`)))
  (if _output_get
    (set `local.CurrentOpenCloseState` false)
    (else
      (set `local.CurrentOpenCloseState` true)))
  (set `self.OpenClosedState` (`local.CurrentOpenCloseState`))
  (return (`self.OpenClosedState`)))

(fn `Unlock`
  (set `self.IsLocked?` false))

(fn `UserConstructionScript`
  (for _array_element (`self.OpenTransforms`)
    (`AddComponent|NODE_AddArrowComponent-0` :`RelativeTransform` _array_element)))